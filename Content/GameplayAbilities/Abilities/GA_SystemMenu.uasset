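; Gameplay ability that opens the pause menu for the owning player and stays active while it is shown.
; Activation pushes WBP_PauseMenu onto the gameplay UI layer and switches input to UI-only, or ends the ability if no valid player controller exists.
; Ending the ability pops the stored widget, restores game-only input with a flush and hides the mouse cursor.
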(event Ability|EventActivateAbility
  (bind _returnvalue (Class|ViperBaseGameplayAbility|GetOwningPlayerController))
  (Utilities|IsValid _returnvalue
    (:Is%20Valid
      (bind _returnvalue_2 (Class|ViperUIBlueprintLibrary|PushContenttoLayerforPlayer _returnvalue "(TagName=\"UI.Layer.Gameplay\")" "/Game/UI/Widgets/Menus/PauseMenu/WBP_PauseMenu.WBP_PauseMenu_C"))
      (bind _output_get (Variables|Default|SetMenuWidget _returnvalue_2))
      (Input|SetInputModeUIOnly _returnvalue _output_get "DoNotLock" false))
    (:Is%20Not%20Valid
      (Ability|EndAbility)
      (Input|SetInputModeGameOnly _returnvalue true)
      (Variables|/Script/Engine.PlayerController|SetbShowMouseCursor _returnvalue false))))

(event Ability|EventOnEndAbility
  (params (bWasCancelled :type Boolean))
  (bind _returnvalue (Class|ViperBaseGameplayAbility|GetOwningPlayerController))
  (bind _menuwidget (Variables|Default|GetMenuWidget)
    (:then
      (Class|ViperUIBlueprintLibrary|PopContentfromLayer _menuwidget)
      (Utilities|IsValid _returnvalue
        (:Is%20Valid
          (Input|SetInputModeGameOnly _returnvalue true)
          (Variables|/Script/Engine.PlayerController|SetbShowMouseCursor _returnvalue false))))
    (:else)))